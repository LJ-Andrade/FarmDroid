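; BP_Tool1 is a rifle-like tool actor that fires projectiles and exposes a second-grip position for the right hand.
; Fire, gated by IsFiring, line-traces forward from the camera when aiming or the muzzle FirePoint otherwise.
; It plays a rifle sound and spawns BP_Projectile at FirePoint, rotated toward the trace hit or end point.
; Tick caches the SecondGripSocket location, which GetRightHandSocketLocation returns.
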(event `self.ReceiveTick`
  (params (DeltaSeconds :type "Float (single-precision)"))
  (`parent.ReceiveTick` DeltaSeconds)
  (set `self.SecondGripLocation` (`SceneComponent.GetSocketLocation` (`self.Tool_Mesh`) "SecondGripSocket")))

(event `/Game/Tools/Interfaces/Int_Tool.Fire`
  (params (Camera :type "SceneComponent Object Reference") (IsAiming :type Boolean))
  (bind _projectilestart (`self.ProjectileStart`))
  (bind _firepoint (`self.FirePoint`))
  (bind _returnvalue (`SceneComponent.K2_GetComponentLocation` (`self.FirePoint`)))
  ;[1 1 1] Fire
  (if (not (`self.IsFiring`))
    (if IsAiming
      (set `self.ProjectileStart` (`SceneComponent.K2_GetComponentLocation` Camera))
      (set `self.ProjectileEnd` (`KismetMathLibrary.GetForwardVector` (`SceneComponent.K2_GetComponentRotation` Camera)))
      (else
        (set `self.ProjectileStart` (`SceneComponent.K2_GetComponentLocation` _firepoint))
        (set `self.ProjectileEnd` (`KismetMathLibrary.GetForwardVector` (`SceneComponent.K2_GetComponentRotation` _firepoint)))))
    (bind (_outhit _returnvalue_2) (`KismetSystemLibrary.LineTraceSingle` _projectilestart (+ _projectilestart (* (`self.ProjectileEnd`) 10000.0)) "TraceTypeQuery1"))
    (`GameplayStatics.PlaySoundAtLocation` "/Game/Sounds/Weapons/SC_RifleFire.SC_RifleFire" (`SceneComponent.K2_GetComponentLocation` (`self.Tool_Mesh`)) (struct) 1.0 1.0 0.0 null null null null)
    (bind (_bblockinghit _binitialoverlap _time _distance _location _impactpoint _normal _impactnormal _physmat _hitactor _hitcomponent _hitbonename _bonename _hititem _elementindex _faceindex _tracestart _traceend) (`GameplayStatics.BreakHitResult` _outhit))
    (`|SpawnActorFromClass` "/Game/Tools/BP_Projectile.BP_Projectile_C" (`KismetMathLibrary.MakeTransform` _returnvalue (`KismetMathLibrary.FindLookAtRotation` _returnvalue (`KismetMathLibrary.SelectVector` _impactpoint _traceend _returnvalue_2))) "Undefined" "OverrideRootScale" null null)))

(fn `GetRightHandSocketLocation`
  (returns (Location :type "Vector Structure"))
  (return (`self.SecondGripLocation`)))

(fn `UserConstructionScript`
  (`parent.UserConstructionScript`))