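; BP_Weapon is a weapon tool actor that fires projectiles and switches between data-driven modes.
; Construction loads mode names from DB_WeaponModes and applies the default; cycling changes the mesh and fire sound.
; Firing line-traces between supplied points, plays the sound and spawns BP_ProjectileBase at FirePoint, aimed at the hit or trace end.
; It also supplies tool type, equip and holster data from DB_Tools, plus a hand IK location.
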(event `self.ReceiveBeginPlay`)

(event `/Game/Tools/_Main/Int_Tool.CycleModeUp`
  (`self.CycleModes` true))

(event `/Game/Tools/_Main/Int_Tool.CycleModeDown`
  (`self.CycleModes` false))

(event `/Game/Tools/_Main/Int_Tool.StartFire1`
  (params (TraceStart :type "Vector Structure") (TraceEnd :type "Vector Structure"))
  ;[1 1 1] Fire
  (if (not (`self.IsFiring`))
    (bind (_outhit _returnvalue) (`KismetSystemLibrary.LineTraceSingle` :`Start` TraceStart :`End` TraceEnd :`TraceChannel` "TraceTypeQuery1" :`DrawDebugType` "ForDuration"))
    (`GameplayStatics.PlaySoundAtLocation` (`self.FireSound`) (`SceneComponent.K2_GetComponentLocation` (`self.ToolMesh`)) (struct) 1.0 1.0 0.0 null null null null)
    (bind (_bblockinghit _binitialoverlap _time _distance _location _impactpoint _normal _impactnormal _physmat _hitactor _hitcomponent _hitbonename _bonename _hititem _elementindex _faceindex _tracestart _traceend) (`GameplayStatics.BreakHitResult` _outhit))
    (`|SpawnActorFromClass` "/Game/Tools/Projectiles/BP_ProjectileBase.BP_ProjectileBase_C" (`KismetMathLibrary.MakeTransform` (`SceneComponent.K2_GetComponentLocation` (`self.FirePoint`)) (`KismetMathLibrary.FindLookAtRotation` (`SceneComponent.K2_GetComponentLocation` (`self.FirePoint`)) (`KismetMathLibrary.SelectVector` _location _traceend _returnvalue))) "AlwaysSpawn" "OverrideRootScale" null null)))

(event `/Game/Tools/_Main/Int_Tool.StopFire1`
  ;[1 1 1] Fire
  (set `self.Firing` false))

(fn `CycleModes`
  (params (CycleUp :type Boolean))
  ;[1 1 1] Cycle Modes
  (bind _newindex (`/Game/_Main/BP_FL_Common.CycleThroughArray` (`KismetArrayLibrary.Array_Length` (`self.WeaponModes`)) (`self.CurrentModeIndex`) CycleUp (`self.LoopModes`)))
  (bind _output_get (set `self.CurrentModeIndex` _newindex))
  (bind _returnvalue (`|GetDataTableRow` "/Game/Tools/_Main/DB_WeaponModes.DB_WeaponModes" (`|GetArrayItem` (`self.WeaponModes`) _output_get))
    (:`then`
      (set `self.CurrentMode` _returnvalue)
      (`self.SelectMode` true))))

(fn `GetRightHandIKTransform`
  (returns (RightHandPosition :type "Vector Structure"))
  (return (`SceneComponent.K2_GetComponentLocation` (`self.IKHand`))))

(fn `GetTool`
  (return))

(fn `GetToolModes`
  (params (Index :type Integer))
  (returns (Name :type Integer) (SKMesh :type "SkeletalMesh Object Reference") (FireSound :type "SoundCue Object Reference") (FireParticle :type "ParticleSystem Object Reference"))
  (return 0 null null null))

(fn `GetToolProperties`
  (returns (Id :type "DataTableRowHandle Structure") (ToolType :type "/Game/Tools/_Main/E_Tool_Type Enum") (SKMesh :type "SkeletalMesh Object Reference") (SocketToEquip :type Name) (HolsterComponent :type Name))
  (bind _returnvalue (`|GetDataTableRow` "/Game/Tools/_Main/DB_Tools.DB_Tools" "Weapon")
    (:`then`
      (bind (_id _tooltype _toolmodes _sockettoequip _holstercomponent) (break `/Game/Tools/_Main/S_Tool_Properties` _returnvalue))
      (return (struct) _tooltype null _sockettoequip _holstercomponent))))

(fn `GetToolType`
  (returns (ToolType :type "/Game/Tools/_Main/E_Tool_Type Enum"))
  (bind _returnvalue (`|GetDataTableRow` "/Game/Tools/_Main/DB_Tools.DB_Tools" "Weapon")
    (:`then`
      (return (`.ToolType_45_8DE32BC8445664092E7CCEADC93C667B` (break `/Game/Tools/_Main/S_Tool_Properties` _returnvalue))))
    (:`RowNotFound`
      (`/Game/_Main/BP_FL_Common.PrintMe` "Row Not Found: " "DB_Weapon@GetToolType"))))

(fn `SelectMode`
  (params (`Select Current` :type Boolean) (RowName :type Name))
  (bind (_id _modename _skmesh _firesound) (break `/Game/Tools/_Main/S_Weapons_Properties` (`self.CurrentMode`)))
  ;[1 1 1] Set Weapon Mode
  (if `Select Current`
    (`/Engine/EditorBlueprintResources/StandardMacros.IsValid` _skmesh
      (:`Is Valid`
        (`SkinnedMeshComponent.SetSkinnedAssetAndUpdate` (`self.ToolMesh`) _skmesh true))
      (:`Is Not Valid`
        _))
    (set `self.FireSound` _firesound)
    (else
      (bind _returnvalue (`|GetDataTableRow` "/Game/Tools/_Main/DB_WeaponModes.DB_WeaponModes" RowName)
        (:`then`
          (bind (_id_2 _modename_2 _skmesh_2 _firesound_2) (break `/Game/Tools/_Main/S_Weapons_Properties` _returnvalue))
          (`/Engine/EditorBlueprintResources/StandardMacros.IsValid` _skmesh_2
            (:`Is Valid`
              (`SkinnedMeshComponent.SetSkinnedAssetAndUpdate` (`self.ToolMesh`) _skmesh_2 true))
            (:`Is Not Valid`
              _))
          (set `self.FireSound` _firesound_2))))))

(fn `UserConstructionScript`
  (`parent.UserConstructionScript`)
  ;[0.1208 0.4677 1] Load Weapon Modes
  (bind _outrownames (`DataTableFunctionLibrary.GetDataTableRowNames` "/Game/Tools/_Main/DB_WeaponModes.DB_WeaponModes"))
  (for _array_element _outrownames
    ;[1 1 1] Set Default Mode
    (`KismetArrayLibrary.Array_Add` (`self.WeaponModes`) _array_element)
    (`self.SelectMode` false (`self.DefaultMode`))))