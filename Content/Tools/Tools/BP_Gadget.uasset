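; BP_Gadget is a Gadget tool actor with a toggleable spotlight flashlight, which starts off at BeginPlay.
; ToggleLight flips the light's visibility and tracks it in FlashLightState.
; GetToolType and GetToolProperties read type, equip socket and holster data from the Gadget row of DB_Tools.
; Firing only prints a Master Tool debug message; mode cycling, GetTool and the right-hand IK getters are empty or placeholder stubs.
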(event `self.ReceiveBeginPlay`
  (`SceneComponent.SetVisibility` (`self.SpotLight`) false false))

(event `/Game/Tools/_Main/Int_Tool.StartFire1`
  (params (TraceStart :type "Vector Structure") (TraceEnd :type "Vector Structure"))
  (`/Game/_Main/BP_FL_Common.PrintMe` "Firing from Master Tool"))

(event `/Game/Tools/_Main/Int_Tool.CycleModeUp`)

(event `/Game/Tools/_Main/Int_Tool.ToggleLight`
  (bind _spotlight (`self.SpotLight`))
  (if (`self.FlashLightState`)
    (`SceneComponent.SetVisibility` _spotlight false false)
    (set `self.FlashLightState` false)
    (else
      (`SceneComponent.SetVisibility` _spotlight true false)
      (set `self.FlashLightState` true))))

(fn `GetRightHandIKTransform`
  (returns (RightHandPosition :type "Vector Structure"))
  (return (0.0 0.0 0.0)))

(fn `GetRightHandSocketLocation`
  (returns (Location :type "Vector Structure"))
  (return (0.0 0.0 0.0)))

(fn `GetTool`
  (return))

(fn `GetToolModes`
  (params (Index :type Integer))
  (returns (Name :type Integer) (SKMesh :type "SkeletalMesh Object Reference") (FireSound :type "SoundCue Object Reference") (FireParticle :type "ParticleSystem Object Reference"))
  (return 0 null null null))

(fn `GetToolProperties`
  (returns (Id :type "DataTableRowHandle Structure") (ToolType :type "/Game/Tools/_Main/E_Tool_Type Enum") (SKMesh :type "SkeletalMesh Object Reference") (SocketToEquip :type Name) (HolsterComponent :type Name))
  (bind _returnvalue (`|GetDataTableRow` "/Game/Tools/_Main/DB_Tools.DB_Tools" "Gadget")
    (:`then`
      (bind (_id _tooltype _toolmodes _sockettoequip _holstercomponent) (break `/Game/Tools/_Main/S_Tool_Properties` _returnvalue))
      (return (struct) _tooltype null _sockettoequip _holstercomponent))))

(fn `GetToolType`
  (returns (ToolType :type "/Game/Tools/_Main/E_Tool_Type Enum"))
  (bind _returnvalue (`|GetDataTableRow` "/Game/Tools/_Main/DB_Tools.DB_Tools" "Gadget")
    (:`then`
      (return (`.ToolType_45_8DE32BC8445664092E7CCEADC93C667B` (break `/Game/Tools/_Main/S_Tool_Properties` _returnvalue))))))

(fn `UserConstructionScript`
  (`parent.UserConstructionScript`))