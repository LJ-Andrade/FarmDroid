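; BP_Tool_Base is the parent Blueprint for tools, providing default stubs that child tools are expected to override.
; Its fire, mode cycling and light toggle events only print debug messages.
; Query functions for tool type, properties, modes and right-hand IK placement return placeholder defaults such as zero vectors and None socket and holster names.
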(event `self.ReceiveBeginPlay`)

(event `/Game/Tools/_Main/Int_Tool.StartFire1`
  (params (TraceStart :type "Vector Structure") (TraceEnd :type "Vector Structure"))
  ;[1 1 1] Fire
  (`KismetSystemLibrary.PrintString` "FIRING 1 From Parent"))

(event `/Game/Tools/_Main/Int_Tool.StopFire1`
  ;[1 1 1] Fire
  (`KismetSystemLibrary.PrintString` "FIRING 1 From Parent"))

(event `/Game/Tools/_Main/Int_Tool.CycleModeUp`
  (`KismetSystemLibrary.PrintString` "CycleMoide From Parent"))

(event `/Game/Tools/_Main/Int_Tool.ToggleLight`
  (`/Game/_Main/BP_FL_Common.PrintMe` "Light Not implementes on this Tool"))

(fn `GetRightHandIKTransform`
  (returns (RightHandPosition :type "Vector Structure"))
  (return (0.0 0.0 0.0)))

(fn `GetRightHandSocketLocation`
  (returns (Location :type "Vector Structure"))
  (return (0.0 0.0 0.0)))

(fn `GetToolModes`
  (params (Index :type Integer))
  (returns (Name :type Integer) (SKMesh :type "SkeletalMesh Object Reference") (FireSound :type "SoundCue Object Reference") (FireParticle :type "ParticleSystem Object Reference"))
  (return 0 null null null))

(fn `GetToolProperties`
  (returns (Id :type "DataTableRowHandle Structure") (ToolType :type "/Game/Tools/_Main/E_Tool_Type Enum") (SKMesh :type "SkeletalMesh Object Reference") (SocketToEquip :type Name) (HolsterComponent :type Name))
  (return (struct) "NewEnumerator0" null "None" "None"))

(fn `GetToolType`
  (returns (ToolType :type "/Game/Tools/_Main/E_Tool_Type Enum"))
  (return "NewEnumerator0"))

(fn `UserConstructionScript`)