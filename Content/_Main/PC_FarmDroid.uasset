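; PC_FarmDroid is the player controller for the farm droid, relaying action inputs to the player pawn.
; On BeginPlay it fetches a player reference through a GetPlayer message on pawn 0 and caches it as PlayerPawn.
; Fire1 press and release start and stop firing, while ToggleTool and ToggleWeapon presses call the pawn's gadget and weapon toggles.
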(event `self.ReceiveBeginPlay`
  ;[1 1 1] Ger Ref To Player
  (bind _playerpawn (message `/Game/FarmDroid/Interfaces/INT_Character.GetPlayer` (`GameplayStatics.GetPlayerPawn` 0)))
  (set `self.PlayerPawn` _playerpawn))

(event `InputAction|Fire1`
  (params (Key :type "Key Structure"))
  (bind _playerpawn (`self.PlayerPawn`))
  ;[1 1 1] Inputs
  ;;[1 0.01705 0] Fire1
  (:`Pressed`
    (`/Game/FarmDroid/Interfaces/INT_Character.StartFiring1` _playerpawn))
  (:`Released`
    (message `/Game/FarmDroid/Interfaces/INT_Character.StopFiring1` _playerpawn)))

(event `InputAction|ToggleTool`
  (params (Key :type "Key Structure"))
  ;[1 1 1] Inputs
  (:`Pressed`
    (`/Game/FarmDroid/Interfaces/INT_Character.ToggleGadget` (`self.PlayerPawn`))))

(event `InputAction|ToggleWeapon`
  (params (Key :type "Key Structure"))
  ;[1 1 1] Inputs
  (:`Pressed`
    (`/Game/FarmDroid/Interfaces/INT_Character.ToggleWeapon` (`self.PlayerPawn`))))

(fn `UserConstructionScript`)