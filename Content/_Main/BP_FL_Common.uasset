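; Blueprint function library of common helpers for debug printing and array index navigation.
; PrintMe joins two strings and prints them with a given duration and key.
; CycleThroughArray steps an index up or down within a given array length, either wrapping around or clamping at the ends based on the Loop flag, and returns the new index.
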(fn `CycleThroughArray`
  (params (ArrayLenght :type Integer) (Index :type "Integer (by ref)") (CycleUp :type Boolean) (Loop :type Boolean))
  (returns (NewIndex :type Integer))
  (locals (CurrentIndex :type Integer))
  (set `local.CurrentIndex` Index)
  (if CycleUp
    ;[1 0.2702 0.3] Cycle Up
    (if (>= (`local.CurrentIndex`) (- (`local.ArrayLenght`) 1))
      (if (`local.Loop`)
        (set `local.CurrentIndex` 0)
        (else
          (bind _result (`/Engine/EditorBlueprintResources/StandardMacros.DecrementInt` (`local.ArrayLenght`))
            (:`  `
              (set `local.CurrentIndex` _result)))))
      (else
        (bind _result_2 (`/Engine/EditorBlueprintResources/StandardMacros.IncrementInt` (`local.CurrentIndex`))
          (:`  `
            (set `local.CurrentIndex` _result_2)))))
    (else
      ;[0.5725 0.6935 1] Cycle Down
      (if (<= (`local.CurrentIndex`) 0)
        (if (`local.Loop`)
          (set `local.CurrentIndex` (- (`local.ArrayLenght`) 1))
          (else
            (set `local.CurrentIndex` 0)))
        (else
          (bind _result_3 (`/Engine/EditorBlueprintResources/StandardMacros.DecrementInt` (`local.CurrentIndex`))
            (:`  `
              (set `local.CurrentIndex` _result_3)))))))
  (return (`local.CurrentIndex`)))

(fn `PrintMe`
  (params (FirstText :type String) (SecondText :type String) (Duration :type "Float (single-precision)" :default 2.0) (Key :type Name))
  (`KismetSystemLibrary.PrintString` null (`KismetStringLibrary.Concat_StrStr` FirstText SecondText) true true (struct :`G` 0.66 :`B` 1.0 :`A` 1.0) Duration Key))